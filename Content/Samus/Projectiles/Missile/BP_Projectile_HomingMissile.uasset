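; Samus's homing missile projectile, handled as a charged projectile through its parent class.
; BeginPlay stops the Missile animation while it waits invisibly, and Shoot restarts it.
; Rotation-follows-velocity is enabled only on firing, so zero velocity during charging doesn't override the arm cannon's rotation.
; If the parent destroys it for insufficient charge, it spawns a regular BP_Projectile_Missile at its transform instead.
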(event `self.ReceiveTick`
  (params (DeltaSeconds :type "Float (single-precision)"))
  (`parent.ReceiveTick` DeltaSeconds))

(event `self.ReceiveBeginPlay`
  ;[1 1 1] right after spawning, missile is invisible. so we stop the animation...
  (`parent.ReceiveBeginPlay`)
  (`SkeletalMeshComponent.Stop` (`self.Missile`)))

(event `self.Shoot`
  (params (`Charge Scale` :type "Float (single-precision)"))
  (bind (_returnvalue_location _returnvalue_rotation) (`KismetMathLibrary.BreakTransform` (`self.GetTransform`)))
  (bind _missile (`self.Missile`))
  (bind _instigator (`self.Instigator`))
  ;[1 1 1] ... just to start it again when we actually shoot
  (`parent.Shoot` `Charge Scale`)
  (`/Engine/EditorBlueprintResources/StandardMacros.IsValid` _missile ; we need an is valid here cuz if we call\ndestroy actor in parent:shoot, blueprint\nthrows an error
    (:`Is Valid`
      (`SkeletalMeshComponent.Play` _missile false)
      ;[1 1 1] since this is treated as a charged projectile, it has a phase in which vel = 0, and this variable (true) overrides actual rotation from arm cannon with 0 rot. so it's false by default until we shoot (missile needs to rotate because homing is not mid!)
      (set `ProjectileMovementComponent.bRotationFollowsVelocity` true (`self.Projectile Movement`)))
    (:`Is Not Valid`
      ;[1 1 1] if the homing missile is being destroyed cause of charge < 100%, just spawn a "normal" variant of a missile
      (`|SpawnActorFromClass` "/Game/Samus/Projectiles/Missile/BP_Projectile_Missile.BP_Projectile_Missile_C" (`KismetMathLibrary.MakeTransform` _returnvalue_location _returnvalue_rotation) "Undefined" "OverrideRootScale" _instigator _instigator))))

(fn `UserConstructionScript`
  (`parent.UserConstructionScript`))
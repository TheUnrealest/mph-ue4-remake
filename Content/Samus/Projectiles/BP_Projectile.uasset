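; Base-style projectile Blueprint for Samus's weapons, handling bounces, impact effects and death on hit.
; Hit counts bounces up to MaxBounces while ProjectileMovement allows bouncing, spawning the optional impact emitter aligned to the surface normal.
; Otherwise it waits DeathDelay and destroys itself, with the impact emitter after that gated by SpawnImpactEffectOnDeath.
; Imperialist spawn, button release and other lifecycle events are empty stubs; a helper prints impact coordinates.
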(event `Spawn Imperialist`
  (params (`Gun Point` :type "Vector Structure") (`Aiming Point` :type "Vector Structure") (`Emitter Normal` :type "Vector Structure")))

(event `self.ReceiveBeginPlay`)

(event `self.ReceiveTick`
  (params (DeltaSeconds :type "Float (single-precision)")))

(event `self.ReceiveHit`
  (params (MyComp :type "PrimitiveComponent Object Reference") (Other :type "Actor Object Reference") (OtherComp :type "PrimitiveComponent Object Reference") (bSelfMoved :type Boolean) (HitLocation :type "Vector Structure") (HitNormal :type "Vector Structure") (NormalImpulse :type "Vector Structure") (Hit :type "HitResult Structure (by ref)"))
  (bind _impact_emitter_template (`self.Impact Emitter Template`))
  (set `self.Hit Location` HitLocation)
  (set `self.Hit Normal` HitNormal)
  ;[1 1 1] should we let the projectile live?
  (if (and (`ProjectileMovementComponent.bShouldBounce` (`self.Projectile Movement`)) (<= (`self.Bounces`) (`self.Max Bounces`)))
    ;[1 1 1] bounce till you're dead
    (`/Engine/EditorBlueprintResources/StandardMacros.IncrementInt` (`self.Bounces`)
      (:`  `
        (`/Engine/EditorBlueprintResources/StandardMacros.IsValid` _impact_emitter_template :!label _label ; if empty, do not use impact emitter
          (:`Is Valid`
            (`GameplayStatics.SpawnEmitterAtLocation` _impact_emitter_template (`self.Hit Location`) (`KismetMathLibrary.MakeRotFromZ` (`self.Hit Normal`)))))))
    (else
      ;[1 1 1] too many bounces? you are ded
      (`KismetSystemLibrary.Delay` (`self.Death Delay`))
      (`self.K2_DestroyActor`)
      (if (`self.Spawn Impact Effect on Death?`)
        (goto _label)))))

(event `self.ReceiveDestroyed`
  ;[1 1 1] when killed, what if we spawn a decal on the impact point? just like the emitter for every hit (and death)
)

(event `Button Released`)

(fn `Show Impact Coordinates`
  (params (`Impact Location` :type "Vector Structure") (`Impact Normal` :type "Vector Structure"))
  (`KismetSystemLibrary.PrintString` (`KismetStringLibrary.Concat_StrStr` "Impact Location: " (`KismetStringLibrary.Conv_VectorToString` `Impact Location`)))
  (`KismetSystemLibrary.PrintString` (`KismetStringLibrary.Concat_StrStr` "Impact Normal: " (`KismetStringLibrary.Conv_VectorToString` `Impact Normal`))))

(fn `UserConstructionScript`)
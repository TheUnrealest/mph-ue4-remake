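; Charged Magmaul projectile Blueprint for Samus, a child of a projectile class that supplies the shooting logic.
; BeginPlay zeroes the projectile movement gravity scale so the projectile is unaffected by gravity until fired.
; Shoot calls the parent with the charge scale, then restores full gravity on the movement component, enabling an arcing shot.
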(event `self.Shoot`
  (params (`Charge Scale` :type "Float (single-precision)"))
  (bind _projectile_movement (`self.Projectile Movement`))
  (`parent.Shoot` `Charge Scale`)
  (`/Engine/EditorBlueprintResources/StandardMacros.IsValid` _projectile_movement
    (:`Is Valid`
      (set `ProjectileMovementComponent.ProjectileGravityScale` 1.0 _projectile_movement))))

(event `self.ReceiveBeginPlay`
  (bind _projectile_movement (`self.Projectile Movement`))
  (`parent.ReceiveBeginPlay`)
  (`/Engine/EditorBlueprintResources/StandardMacros.IsValid` _projectile_movement
    (:`Is Valid`
      (set `ProjectileMovementComponent.ProjectileGravityScale` 0.0 _projectile_movement))))

(fn `UserConstructionScript`
  (`parent.UserConstructionScript`))
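; Charged Samus projectile that starts invisible and inert while charging, then Shoot scales, detaches and launches it with charge-scaled damage, or destroys it below a threshold.
; Its lifespan timer starts on release rather than on spawn.
; Homing variants sphere-trace forward on a channel chosen by trace type, lock onto the targetable character hit, and set acceleration by distance.
; Tick drops the target when speed falls, indicating a miss.
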(event `Shoot`
  (params (`Charge Scale` :type "Float (double-precision)"))
  (bind _returnvalue (`self.K2_GetActorLocation`))
  (bind _projectile_movement (`self.Projectile Movement`))
  ;[1 1 1] full detach & effect tweaking procedure! wait, stop the procedure! did i say procedure? operation? ofc not a reference to a really random surgery game for ds and wii
  (if (>= `Charge Scale` (`self.Scale Threshold`))
    (`self.SetActorScale3D` (`KismetMathLibrary.Conv_DoubleToVector` `Charge Scale`)) ; ... but then it grows (that's what I told Anna,\nspoiler: she enjoyed every 3D scale of it)
    (`PrimitiveComponent.SetCollisionEnabled` (`self.Collision`) "QueryAndPhysics")
    (`ProjectileMovementComponent.SetVelocityInLocalSpace` (`self.Projectile Movement`) (`KismetMathLibrary.MakeVector` (`self.Projectile Velocity`)))
    (`self.K2_DetachFromActor` "KeepWorld" "KeepWorld" "KeepWorld") ; and after growing it comes out (yes, that's what I told Anna too\neven tho she wanted something called "creampie" but idk i never baked something)
    (set `self.Calculated Damage` (`KismetMathLibrary.FTrunc` (* (`self.Damage`) `Charge Scale`))) ; haha i love dirty jokes
    (`ActorComponent.Activate` (`self.Particle System`) true) ; and full particle we go!
    (`KismetSystemLibrary.K2_SetTimerDelegate` (delegate `Kill Projectile (Timer Only)`) (`self.Projectile Lifespan`)) ; right after shooting we set a timer which is the lifespan\nof the projectile. we cannot do that using InitialLifespan\nin class settings cuz if you try, countdown will start when\ncharging. we want this countdown to start after releasing\nthe projectile from charging
    (set `self.Emitter Scale` (`KismetMathLibrary.Conv_DoubleToVector` `Charge Scale`))
    ;[1 1 1] homing components for energy beam, volt driver and... yes, missiles. (homing missiles are treated just like charged projectiles, minus scaling over time and effects)
    (if (`ProjectileMovementComponent.bIsHomingProjectile` (`self.Projectile Movement`))
      (bind (_outhit _returnvalue_2) (`KismetSystemLibrary.SphereTraceSingle` _returnvalue (+ _returnvalue (* (`self.GetActorForwardVector`) (`self.Homing Trace Length`))) (`self.Homing Radius`) (select `/Game/Samus/Projectiles/Common/Data/E_HomingTraces` (`self.Homing Trace Type`) :`NewEnumerator0` "TraceTypeQuery3" :`NewEnumerator1` "TraceTypeQuery5" :`NewEnumerator2` "TraceTypeQuery6" :!type "ETraceTypeQuery Enum") false (`|MakeArray` (`self.Instigator`) :!type "Actor Object Reference") "None" true (struct :`R` 1.0 :`A` 1.0) (struct :`G` 1.0 :`A` 1.0) 3.0)) ; Homing Player Trace: follow players only. (Missile, Volt Driver)\nHoming Object Trace: follow objects only.\nHoming Player and Object Trace: follow both players and objects. Whatever\nis hit first, will be the only target. (Energy Beam)
      (if _returnvalue_2
        (bind _asshootin_guy_gurl (cast `/Game/Samus/BP_TargetableCharacter` (`.HitActor` (`GameplayStatics.BreakHitResult` _outhit))))
        (set `ProjectileMovementComponent.HomingTargetComponent` (`/Game/Samus/BP_TargetableCharacter.BPC_HomingProjectile_Target` _asshootin_guy_gurl) _projectile_movement) ; we set the target of this projectile...
        (set `ProjectileMovementComponent.HomingAccelerationMagnitude` (`KismetMathLibrary.Lerp` (`self.Homing Accel Max`) (`self.Homing Accel Min`) (/ (`.Distance` (`GameplayStatics.BreakHitResult` _outhit)) (`self.Homing Trace Length`))) _projectile_movement) ; ... and its acceleration.
      ))
    (else
      (`self.K2_DestroyActor`))))

(event `Kill Projectile (Timer Only)`
  ;[1 1 1] full detach & effect tweaking procedure! wait, stop the procedure! did i say procedure? operation? ofc not a reference to a really random surgery game for ds and wii
  (`self.K2_DestroyActor`))

(event `self.ReceiveBeginPlay`
  (`parent.ReceiveBeginPlay`)
  ;[1 1 1] initial spawn
  (`self.SetActorScale3D` (0.0 0.0 0.0)) ; it starts very tiny (invisible), cuz we just want\nthe particle system reference...
  (`PrimitiveComponent.SetCollisionEnabled` (`self.Collision`) "NoCollision")
  (`ActorComponent.Deactivate` (`self.Particle System`)) ; this will prevent the particle system from simulating. setting the scale to 1 will pop in some particles without this
)

(event `self.ReceiveTick`
  (params (DeltaSeconds :type "Float (single-precision)"))
  (`parent.ReceiveTick` DeltaSeconds)
  ;[1 1 1] homing target detach, in case of failed approach (fsx overspeed noise)
  (`/Engine/EditorBlueprintResources/StandardMacros.IsValid` (`ProjectileMovementComponent.HomingTargetComponent` (`self.Projectile Movement`)) ; proceed only if we actually set a homing target
    (:`Is Valid`
      (if (<= (`KismetMathLibrary.VSize` (`self.GetVelocity`)) 1000.0)
        (set `ProjectileMovementComponent.HomingTargetComponent` null (`self.Projectile Movement`)) ; we set this to null, it works!
      ))))

(fn `UserConstructionScript`
  (`parent.UserConstructionScript`))
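; Charged Judicator shot for Samus's arm cannon, acting as a short-lived spawner for a shotgun-like burst of normal Judicator projectiles.
; Shoot replaces the parent logic: at or above the charge threshold it spawns sub-projectiles with random pitch and yaw spread, then scales them by charge.
; It delays self-destruction so the arm cannon still sees a valid projectile for camera shake.
; Below the threshold it destroys itself immediately, spawning nothing.
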(event `self.Shoot`
  (params (`Charge Scale` :type "Float (single-precision)"))
  (bind _returnvalue (`self.GetTransform`))
  (bind _rotation_delta (`self.Rotation Delta`))
  ;[1 1 1] since we ain't using the full parent:shoot, i just wrote again this very important code (VIC)
  (if (>= `Charge Scale` (`self.Scale Threshold`))
    ;[1 1 1] we spawn a number of x sub projectiles (normal judicator) with partially randomized rotation (shotgun-like) (fortnite accuracy 0% lol) (drum shotgun)
    (for _ (range 1 (+ (`self.Projectiles To Spawn`) 1))
      (bind _returnvalue_2 (`|SpawnActorFromClass` "/Game/Samus/Projectiles/Judicator/BP_Projectile_Judicator.BP_Projectile_Judicator_C" (`KismetMathLibrary.MakeTransform` (.location _returnvalue) (`KismetMathLibrary.MakeRotator` (.roll (.rotation _returnvalue)) (+ (* (`KismetMathLibrary.RandomFloatInRange` -1.0 1.0) _rotation_delta) (.pitch (.rotation _returnvalue))) (+ (* (`KismetMathLibrary.RandomFloatInRange` -1.0 1.0) _rotation_delta) (.yaw (.rotation _returnvalue)))) (.scale _returnvalue)) "Undefined" "OverrideRootScale" null (`GameplayStatics.GetPlayerCharacter` 0)))
      (`KismetArrayLibrary.Array_Add` (`self.Sub Projectiles Spawned`) _returnvalue_2) ; we store the references\nhere in this array
    )
    ;[1 1 1] also we apply the scaling method from charged beams
    (for _array_element (`self.Sub Projectiles Spawned`)
      (`self.SetActorScale3D` _array_element (`KismetMathLibrary.Conv_DoubleToVector` (* `Charge Scale` (`self.Sub Projectile Scale`)))))
    (`KismetSystemLibrary.Delay` (`self.Death Delay`)) ; this will keep the projectile valid enough\nfor the arm cannon to process the "validness"\nand execute a camera shake
    (`self.K2_DestroyActor`)
    (else
      (`self.K2_DestroyActor`))))

(event `self.ReceiveBeginPlay`
  (`parent.ReceiveBeginPlay`))

(fn `UserConstructionScript`
  (`parent.UserConstructionScript`))
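; Imperialist projectile for Samus: an instant beam shot visual with an impact effect and decal.
; SpawnImperialist receives gun point, aim point and surface normal from the caller, reusing the aim-adjust trace rather than tracing again.
; It stretches two beam emitters between the points, then spawns the impact emitter and a randomly scaled, rolled decal that fades out.
; The decal logic is deliberately copied from the base projectile Blueprint.
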(event `self.Spawn Imperialist`
  (params (`Gun Point` :type "Vector Structure") (`Aiming Point` :type "Vector Structure") (`Emitter Normal` :type "Vector Structure"))
  (bind (_returnvalue_roll _returnvalue_pitch _returnvalue_yaw) (`KismetMathLibrary.BreakRotator` (`KismetMathLibrary.Conv_VectorToRotator` `Emitter Normal`)))
  (bind _particle_system (`self.Particle System`))
  ;[1 1 1] calibrate the imperialist using the aim adjust trace, instead of doing another one each time we shoot. uses a little bit more of memory (like, 15 bytes?)
  (`parent.ReceiveBeginPlay`)
  (`ParticleSystemComponent.SetBeamSourcePoint` _particle_system 0 `Gun Point` 0)
  (`ParticleSystemComponent.SetBeamTargetPoint` _particle_system 0 `Aiming Point` 0)
  (`ParticleSystemComponent.SetBeamSourcePoint` _particle_system 1 `Gun Point` 0)
  (`ParticleSystemComponent.SetBeamTargetPoint` _particle_system 1 `Aiming Point` 0)
  ;[1 1 1] impact emitter brrrrrr!111!11 and also decal
  (bind _output_get (set `self.Hit Location` `Aiming Point`))
  (`GameplayStatics.SpawnEmitterAtLocation` (`self.Impact Emitter Template`) _output_get (`KismetMathLibrary.MakeRotFromZ` `Emitter Normal`))
  (bind _returnvalue (`GameplayStatics.SpawnDecalAtLocation` (`self.Decal Material`) (* (25.0 25.0 25.0) (* (`self.Decal Scale`) (`KismetMathLibrary.RandomFloatInRange` (- 1.0 (`self.Decal Scale Variation`)) 1.0))) _output_get (`KismetMathLibrary.MakeRotator` (`KismetMathLibrary.RandomFloatInRange` 0.0 360.0) _returnvalue_pitch _returnvalue_yaw) (`self.Decal Lifespan`))) ; 15000 iq move: did you see i blatantly copied and pasted the decal code?\n\nyep, its on purpose!\nnormally this bp would inherit behaviour from bp projectile. the decal, according\nto the parent, would be scaled accordingly to the "collision cylinder" but in here\nthat scale is zero = no effects bruh!!!\n\nimagine adding an entire check so that imperialist would override that...\n\nor\n\ndo not inherit event hit (it is literally at begin play)
  (`DecalComponent.SetFadeOut` _returnvalue (`self.Decal Fadeout Delay`) (`self.Decal Fadeout Duration`) true) ; unfortunately, there's no faster way\nyou need to set it up for each dynamic component\n\nand martina it out from the game when it becomes transparent
)

(fn `UserConstructionScript`
  (`parent.UserConstructionScript`))
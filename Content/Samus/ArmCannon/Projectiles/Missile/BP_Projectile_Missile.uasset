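; Missile projectile for Samus's arm cannon that flies at its initial speed, then accelerates after a short delay.
; BeginPlay waits one second before opening a Gate that Tick feeds every frame.
; While the gate is open, SpeedAlpha accumulates delta time to ease local forward velocity from InitialSpeed to MaxSpeed on the ProjectileMovement component.
; The gate closes once the roughly one-second ramp completes.
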(event `self.ReceiveBeginPlay`
  (bind _projectile_movement (`self.Projectile Movement`))
  (`parent.ReceiveBeginPlay`)
  (`KismetSystemLibrary.Delay` 1.0)
  (goto _label :!via `Open`))

(event `self.ReceiveTick`
  (params (DeltaSeconds :type "Float (single-precision)"))
  (bind _projectile_movement (`self.Projectile Movement`))
  (bind _returnvalue (+ DeltaSeconds (`self.Speed Alpha`)))
  (`parent.ReceiveTick` DeltaSeconds)
  (`/Engine/EditorBlueprintResources/StandardMacros.Gate` true :!label _label
    (:`Exit`
      (set `self.Speed Alpha` _returnvalue)
      (`ProjectileMovementComponent.SetVelocityInLocalSpace` (`self.Projectile Movement`) (`KismetMathLibrary.MakeVector` (`|EaseFunction` "EaseInOut" _returnvalue (`ProjectileMovementComponent.InitialSpeed` _projectile_movement) (`ProjectileMovementComponent.MaxSpeed` _projectile_movement))))
      (if (>= (`self.Speed Alpha`) 1.0)
        (goto _label :!via `Close`)))))

(fn `UserConstructionScript`
  (`parent.UserConstructionScript`))
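; BP_Projectile_Imperialist is the beam shot for the Imperialist in Samus's arm cannon.
; SpawnImperialist stretches two beam emitters from the gun point to the aiming point, then spawns an impact effect there, oriented to the surface normal.
; It takes the hit point from the existing aim-adjust trace instead of tracing per shot, and has no active tick or overlap logic of its own.
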(event `self.Spawn Imperialist`
  (params (`Gun Point` :type "Vector Structure") (`Aiming Point` :type "Vector Structure") (`Emitter Normal` :type "Vector Structure"))
  (bind _particle_system (`self.Particle System`))
  ;[1 1 1] calibrate the imperialist using the aim adjust trace, instead of doing another one each time we shoot. uses a little bit more of memory (like, 15 bytes?)
  (`parent.ReceiveBeginPlay`)
  (`ParticleSystemComponent.SetBeamSourcePoint` _particle_system 0 `Gun Point` 0)
  (`ParticleSystemComponent.SetBeamTargetPoint` _particle_system 0 `Aiming Point` 0)
  (`ParticleSystemComponent.SetBeamSourcePoint` _particle_system 1 `Gun Point` 0)
  (`ParticleSystemComponent.SetBeamTargetPoint` _particle_system 1 `Aiming Point` 0)
  ;[1 1 1] impact emitter brrrrrr!111!11
  (bind _output_get (set `self.Hit Location` `Aiming Point`))
  (`GameplayStatics.SpawnEmitterAtLocation` (`self.Impact Emitter Template`) _output_get (`KismetMathLibrary.MakeRotFromZ` `Emitter Normal`)))

(fn `UserConstructionScript`
  (`parent.UserConstructionScript`))
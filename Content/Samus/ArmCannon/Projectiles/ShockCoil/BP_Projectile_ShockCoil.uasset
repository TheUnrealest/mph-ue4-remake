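; Shock Coil beam projectile that attaches to Samus's gameplay gun and is destroyed when the button is released.
; Each tick, a forward sphere trace on the channel shared by surfaces and players provides auto-aim for the beam.
; The beam endpoint locks onto a targetable character's Shock Coil target, stops at other hits, or extends to full range.
; An impact particle system follows that endpoint.
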(event `self.ReceiveBeginPlay`
  (`parent.ReceiveBeginPlay`)
  (bind _asbp_samus (cast `/Game/Samus/Blueprints/BP_Samus` (`self.Instigator`)))
  (`self.K2_AttachToComponent` (`/Game/Samus/Blueprints/BP_Samus.Gameplay Gun` _asbp_samus) "None" "SnapToTarget" "SnapToTarget" "SnapToTarget"))

(event `self.ReceiveTick`
  (params (DeltaSeconds :type "Float (single-precision)"))
  (bind _returnvalue (`self.GetActorForwardVector`))
  (bind _returnvalue_2 (+ (`self.K2_GetActorLocation`) (* _returnvalue (`self.Trace Offset`))))
  (bind _returnvalue_3 (+ (* _returnvalue (`self.Trace Length (Beam Range)`)) _returnvalue_2))
  (`parent.ReceiveTick` DeltaSeconds)
  (if (not (`self.IsActorBeingDestroyed`))
    ;[1 1 1] sphere trace. it works on the shock coil trace channel, in which both surfaces and players respond
    (bind (_outhit _returnvalue_4) (`KismetSystemLibrary.SphereTraceSingle` _returnvalue_2 _returnvalue_3 (`self.Trace Radius (Beam Auto Aim Range)`) "TraceTypeQuery4" true))
    ;[1 1 1] did we kaboom something?
    (if _returnvalue_4
      ;[1 1 1] if we did, let's actually test if we're hitting a player or not (it can also be a block all surface bruh)
      (bind _asshootin_guy_gurl (cast `/Game/Samus/BP_TargetableCharacter` (`.HitActor` (`GameplayStatics.BreakHitResult` _outhit))) ; this is gonna be veeeeeery unoptimized
        (:`then`
          (bind _returnvalue_5 (`SceneComponent.K2_GetComponentLocation` (`/Game/Samus/BP_TargetableCharacter.BPC_ShockCoil_Target` _asshootin_guy_gurl)))
          ;[1 1 1] if the hit thingy is a player, just use the shock coil target to literally lock the beam onto the player
          (`ParticleSystemComponent.SetBeamTargetPoint` (`self.Particle System`) 0 _returnvalue_5 0)
          ;[1 0.1305 0.07081] unoptimized method to create impact effect: snap the impact particle system to the beam target point
          (`SceneComponent.K2_SetWorldLocation` (`self.Impact Particle System`) _returnvalue_5 false false))
        (:`CastFailed`
          ;[1 1 1] if it's not a player, just crop the beam to the impact point so it doesn't xray all over the place
          (`ParticleSystemComponent.SetBeamTargetPoint` (`self.Particle System`) 0 (`.Location` (`GameplayStatics.BreakHitResult` _outhit)) 0)
          (`SceneComponent.K2_SetWorldLocation` (`self.Impact Particle System`) (`.Location` (`GameplayStatics.BreakHitResult` _outhit)) false false)))
      (else
        ;[1 1 1] if we didn't hit anything just set the beam target to the end
        (`ParticleSystemComponent.SetBeamTargetPoint` (`self.Particle System`) 0 _returnvalue_3 0)
        (`SceneComponent.K2_SetWorldLocation` (`self.Impact Particle System`) _returnvalue_3 false false)))))

(event `self.Button Released`
  (`self.K2_DestroyActor`))

(fn `UserConstructionScript`
  (`parent.UserConstructionScript`))
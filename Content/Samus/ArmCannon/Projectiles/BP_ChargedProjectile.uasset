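; Charged projectile for Samus's arm cannon that starts attached, hidden at zero scale with collision and particles off.
; Shoot destroys it if the charge scale is below a threshold; otherwise it scales up, enables collision, launches along local X and detaches.
; Damage scales with the charge and is truncated to a whole number.
; Particles stay deactivated until firing to avoid popping in when the scale changes.
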(event `Shoot`
  (params (`Charge Scale` :type "Float (double-precision)"))
  (if (>= `Charge Scale` (`self.Scale Threshold`))
    (`self.SetActorScale3D` (`KismetMathLibrary.Conv_DoubleToVector` `Charge Scale`)) ; ... but then it grows (that's what I told Anna,\nspoiler: she enjoyed every 3D scale of it)
    (`PrimitiveComponent.SetCollisionEnabled` (`self.Collision`) "QueryAndPhysics")
    (`ProjectileMovementComponent.SetVelocityInLocalSpace` (`self.Projectile Movement`) (`KismetMathLibrary.MakeVector` (`self.Projectile Velocity`)))
    (`self.K2_DetachFromActor` "KeepWorld" "KeepWorld" "KeepWorld") ; and after growing it comes out (yes, that's what I told Anna too\neven tho she wanted something called "creampie" but idk i never baked something)
    (set `self.Calculated Damage` (`KismetMathLibrary.FTrunc` (* (`self.Damage`) `Charge Scale`))) ; haha i love dirty jokes
    (`ActorComponent.Activate` (`self.Particle System`) true) ; and full particle we go!
    (else
      (`self.K2_DestroyActor`))))

(event `self.ReceiveBeginPlay`
  (`parent.ReceiveBeginPlay`)
  (`self.SetActorScale3D` (0.0 0.0 0.0)) ; it starts very tiny (invisible), cuz we just want\nthe particle system reference...
  (`PrimitiveComponent.SetCollisionEnabled` (`self.Collision`) "NoCollision")
  (`ActorComponent.Deactivate` (`self.Particle System`)) ; this will prevent the particle system from simulating. setting the scale to 1 will pop in some particles without this
)

(fn `UserConstructionScript`
  (`parent.UserConstructionScript`))
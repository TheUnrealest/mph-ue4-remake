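; Player pawn for Samus's morph form, moved as a physics body with camera-relative controls.
; Movement input applies acceleration forces to the capsule along the camera's flattened forward and right vectors, then clamps horizontal velocity to a maximum speed.
; Look input drives controller yaw and pitch, and Jump adds an upward velocity impulse without a ground check.
; The per-tick movement update is empty, and the downward in-air trace is left disconnected.
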(event `self.ReceiveTick`
  (params (DeltaSeconds :type "Float (single-precision)"))
  (`self.Update Movement Variables`))

(event `InputAxis|MoveForward` :overrideparent false
  (params (AxisValue :type "Float (single-precision)"))
  (bind _capsulecomponent (`self.CapsuleComponent`))
  (bind (_returnvalue_x _returnvalue_y) (`KismetMathLibrary.BreakVector` (`SceneComponent.GetForwardVector` (`self.Camera`))))
  (`PrimitiveComponent.AddForce` _capsulecomponent (* (`KismetMathLibrary.Vector_Normal2D` (`KismetMathLibrary.MakeVector` _returnvalue_x _returnvalue_y)) (* AxisValue 5000.0)) "None" true)
  (bind _returnvalue (`PrimitiveComponent.GetPhysicsLinearVelocity` _capsulecomponent "None" :!label _label))
  (bind _output_get (set `self.Velocity` (`KismetMathLibrary.Vector_ClampSize2D` _returnvalue 0.0 850.0)))
  (`PrimitiveComponent.SetPhysicsLinearVelocity` _capsulecomponent _output_get false "None"))

(event `InputAxis|MoveRight` :overrideparent false
  (params (AxisValue :type "Float (single-precision)"))
  (bind (_returnvalue_x _returnvalue_y) (`KismetMathLibrary.BreakVector` (`SceneComponent.GetRightVector` (`self.Camera`))))
  (`PrimitiveComponent.AddForce` (`self.CapsuleComponent`) (* (`KismetMathLibrary.Vector_Normal2D` (`KismetMathLibrary.MakeVector` _returnvalue_x _returnvalue_y)) (* AxisValue 5000.0)) "None" true)
  (goto _label))

(event `Update Movement Variables`)

(event `InputAxis|Turn` :overrideparent false
  (params (AxisValue :type "Float (single-precision)"))
  (`self.AddControllerYawInput` AxisValue))

(event `InputAxis|TurnRate`
  (params (AxisValue :type "Float (single-precision)"))
  (`self.AddControllerYawInput` AxisValue))

(event `InputAxis|LookUpRate`
  (params (AxisValue :type "Float (single-precision)"))
  (`self.AddControllerPitchInput` AxisValue))

(event `InputAxis|LookUp` :overrideparent false
  (params (AxisValue :type "Float (single-precision)"))
  (`self.AddControllerPitchInput` AxisValue))

(event `InputAction|Jump`
  (params (Key :type "Key Structure"))
  (:`Pressed`
    (`PrimitiveComponent.AddImpulse` (`self.CapsuleComponent`) (0.0 0.0 350.0) "None" true)))

(fn `UserConstructionScript`)
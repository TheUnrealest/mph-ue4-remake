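; HUD Blueprint for Samus that draws the aiming crosshair on screen, hidden while the character is morphed.
; On BeginPlay it caches the player's BP_Samus, then each DrawHUD centers a texture on that character's CrosshairScreenLocation.
; The crosshair turns red when the character's AimHitActor is a BP_TargetableCharacter or subclass, and is otherwise faint white.
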(event `self.ReceiveBeginPlay`
  (bind _assamos (cast `/Game/Samus/Blueprints/BP_Samus` (`GameplayStatics.GetPlayerCharacter` 0)))
  (set `self.Character Reference!` _assamos))

(event `self.ReceiveDrawHUD`
  (params (SizeX :type Integer) (SizeY :type Integer))
  (bind _character_reference_ (`self.Character Reference!`))
  (bind (_crosshair_screen_location_x _crosshair_screen_location_y) (`KismetMathLibrary.BreakVector2D` (`/Game/Samus/Blueprints/BP_Samus.Crosshair Screen Location` _character_reference_)))
  (if (not (`/Game/Samus/Blueprints/BP_Samus.Is Morphed?` _character_reference_))
    (`self.DrawTexture` "/Game/Samus/Blueprints/T_HUD.T_HUD" (- _crosshair_screen_location_x 32.0) (- _crosshair_screen_location_y 32.0) 64.0 64.0 0.0 0.0 1.0 1.0 (select `bool` (`KismetMathLibrary.ClassIsChildOf` (`GameplayStatics.GetObjectClass` (`/Game/Samus/Blueprints/BP_Samus.Aim Hit Actor` _character_reference_)) "/Game/Samus/BP_TargetableCharacter.BP_TargetableCharacter_C") :`false` (struct :`R` 1.0 :`G` 1.0 :`B` 1.0 :`A` 0.2) :`true` (struct :`R` 1.0 :`G` 0.148863 :`B` 0.069179 :`A` 1.0) :!type "LinearColor Structure"))))

(fn `UserConstructionScript`)